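; Omen player character Blueprint, with most ability logic left in disconnected graphs and BeginPlay and Tick empty, marked as CPP.
; CameraModeLevel drops the actor far below the level and spawns a BP_MH_Omen_copy stand-in at its old transform; PlayerModeLevel teleports back to the copy and destroys it.
; The unexecuted graphs hold Q projectile, E camera-steered sphere and C trace-guided teleport skills.
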(event `CustomEvent` :!signature `self.OnDestroyed`
  (params (DestroyedActor :type "Actor Object Reference"))
  ;[1 1 1] 카메라 위치에서 구체 생성
)

(event `Key|LeftMouseButton`
  (params (Key :type "Key Structure")))

(event `self.ReceiveBeginPlay`)

(event `Key|R`
  (params (Key :type "Key Structure")))

(event `EnhancedInput|/Game/ThirdPerson/Input/Actions/IA_Key_C`
  (params (ActionValue :type Boolean) (ElapsedSeconds :type "Float (double-precision)") (TriggeredSeconds :type "Float (double-precision)") (InputAction :type "InputAction Object Reference" :default "/Game/ThirdPerson/Input/Actions/IA_Key_C.IA_Key_C"))
  ;[1 1 1] CPP
)

(event `Key|RightMouseButton`
  (params (Key :type "Key Structure")))

(event `Key|LeftMouseButton`
  (params (Key :type "Key Structure"))
  ;[1 1 1] CPP
)

(event `self.ReceiveTick`
  (params (DeltaSeconds :type "Float (single-precision)")))

(event `self.CameraModeLevel`
  (bind _output_get (set `self.New Relative Location` (`self.K2_GetActorLocation`)))
  (`self.K2_SetActorLocation` (- _output_get (0.0 0.0 15000.0)) false true)
  (bind _returnvalue (`|SpawnActorFromClass` "/Game/LMH/BP/BP_MH_Omen_copy.BP_MH_Omen_copy_C" (`KismetMathLibrary.MakeTransform` _output_get (`self.K2_GetActorRotation`) (`self.GetActorScale3D`)) "Undefined" "MultiplyWithRoot" null null))
  (set `self.CopyPlayer` _returnvalue))

(event `self.PlayerModeLevel`
  (bind _copyplayer (`self.CopyPlayer`))
  (`/Engine/EditorBlueprintResources/StandardMacros.IsValid` _copyplayer
    (:`Is Valid`
      (`self.K2_SetActorLocationAndRotation` (`self.K2_GetActorLocation` _copyplayer) (`self.K2_GetActorRotation` _copyplayer) false true)
      (`self.K2_DestroyActor` _copyplayer))))

(event `OnDestroyed_Event` :!signature `self.OnDestroyed`
  (params (DestroyedActor :type "Actor Object Reference")))

(fn `Spawn NSH2`)

(fn `UserConstructionScript`)