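; BP_NSHHH is an actor Blueprint that, as wired, only prints a debug string on BeginPlay.
; Its ToButtom custom events, overlap and Tick are empty.
; Disconnected nodes hold an unfinished move-to-bottom behavior: a visibility trace along the actor's vertical axis picks one of two timelines, lerping the actor to the hit point or trace end.
; A disconnected EndLifeTime timer and debug prints also never run.
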(event `self.ReceiveBeginPlay`
  (`KismetSystemLibrary.PrintString` "nasun bieing"))

(event `self.ReceiveTick`
  (params (DeltaSeconds :type "Float (single-precision)")))

(event `ToButtom_1`)

(event `self.ToButtomMH`)

(event `self.ToButtomMHBabo`)

(fn `UserConstructionScript`)