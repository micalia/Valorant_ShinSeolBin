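; BP_Nassunhawn is an actor with a ToButtom event that moves it along a vertical line, apparently to drop it to the bottom.
; A visibility trace at its current X and Y, drawn persistently for debugging, picks the impact point or, on a miss, the trace end.
; Separate timelines lerp it there from its updated location; only the miss branch then schedules EndLifeTime after LifeTime, a function not defined here.
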(event `self.ToButtom`
  (bind (_returnvalue_x _returnvalue_y) (`KismetMathLibrary.BreakVector` (`self.K2_GetActorLocation`)))
  (`KismetSystemLibrary.PrintString` "tobottom")
  (bind (_outhit _returnvalue) (`KismetSystemLibrary.LineTraceSingle` :`Start` (`self.K2_GetActorLocation`) :`End` (`KismetMathLibrary.MakeVector` _returnvalue_x _returnvalue_y) :`TraceChannel` "TraceTypeQuery1" :`DrawDebugType` "Persistent"))
  (if _returnvalue
    (bind (_direction _newtrack_0) (`Timeline|Timeline_0`)
      (:`Update`
        (`self.K2_SetActorLocation` (`KismetMathLibrary.VLerp` (`self.K2_GetActorLocation`) (`.ImpactPoint` (`GameplayStatics.BreakHitResult` _outhit)) _newtrack_0))))
    (else
      (bind (_direction_2 _newtrack_0_2) (`Timeline|Timeline`)
        (:`Update`
          (`self.K2_SetActorLocation` (`KismetMathLibrary.VLerp` (`self.K2_GetActorLocation`) (`.TraceEnd` (`GameplayStatics.BreakHitResult` _outhit)) _newtrack_0_2)))
        (:`Finished`
          (`KismetSystemLibrary.K2_SetTimer` null "EndLifeTime" (`self.LifeTime`)))))))

(fn `UserConstructionScript`)