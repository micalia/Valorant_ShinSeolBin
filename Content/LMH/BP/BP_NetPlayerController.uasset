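; Player controller for a networked game that shows whether it runs as server or client and supports switching the possessed pawn.
; A second after BeginPlay it creates a status widget labelled Server or Client based on authority.
; ChangePawn calls ServerChangePawn, which possesses the given pawn, then calls MulticastEnableInput to enable input on it for the local controller, with debug prints along the way.
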(event `self.ReceiveBeginPlay`
  (`KismetSystemLibrary.Delay` 1.0)
  (if (`self.HasAuthority`)
    (bind _returnvalue (`|CreateWidget` "/Game/SB/UMG/WB_ChkCurrStatus.WB_ChkCurrStatus_C"))
    (bind _chkservertxt (`/Game/SB/UMG/WB_ChkCurrStatus.ChkServerTxt` _returnvalue))
    (`/Engine/EditorBlueprintResources/StandardMacros.IsValid` _chkservertxt
      (:`Is Valid`
        (`UserWidget.AddToViewport` _returnvalue 0)
        (set `TextBlock.Text` (`KismetTextLibrary.Conv_StringToText` "Server") _chkservertxt)
        (`KismetSystemLibrary.PrintString` "Server")))
    (else
      (bind _returnvalue_2 (`|CreateWidget` "/Game/SB/UMG/WB_ChkCurrStatus.WB_ChkCurrStatus_C"))
      (`UserWidget.AddToViewport` _returnvalue_2 0)
      (bind _chkservertxt_2 (`/Game/SB/UMG/WB_ChkCurrStatus.ChkServerTxt` _returnvalue_2))
      (`/Engine/EditorBlueprintResources/StandardMacros.IsValid` _chkservertxt_2
        (:`Is Valid`
          (set `TextBlock.Text` (`KismetTextLibrary.Conv_StringToText` "Client") _chkservertxt_2)
          (`KismetSystemLibrary.PrintString` "Client"))))))

(event `ServerChangePawn`
  (params (MyPawn :type "BaseCharacter Object Reference"))
  (`self.Possess` MyPawn)
  (`KismetSystemLibrary.PrintString` "Re Possess")
  (`self.MulticastEnableInput` MyPawn))

(event `MulticastEnableInput`
  (params (MyPawn :type "BaseCharacter Object Reference"))
  (if (`self.IsLocalPlayerController`)
    (`self.EnableInput` MyPawn self)
    (`KismetSystemLibrary.PrintString` "Enable Input!!!!!!!!!!!!!!!!!!!!")))

(fn `ChangePawn`
  (params (Character :type "BaseCharacter Object Reference"))
  (`self.ServerChangePawn` Character))

(fn `UserConstructionScript`)