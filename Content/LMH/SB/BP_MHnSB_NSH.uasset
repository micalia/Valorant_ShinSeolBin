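; Short-lived smoke actor that drops toward the ground when ToButtomMH is called, removing itself 10 seconds after BeginPlay.
; ToButtomMH calls ServerSomething, which spawns the Smoke_MH effect at the actor's position and line-traces vertically from there, keeping X and Y.
; One of two timelines then lerps the actor from its current location to the impact point, or to the trace end on a miss.
; Several disconnected smoke, timer and debug nodes never run.
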(event `self.ReceiveBeginPlay`
  (`self.SetLifeSpan` 10.0))

(event `self.ToButtomMH`
  (`self.ServerSomething`))

(event `ServerSomething`
  (bind (_returnvalue_x _returnvalue_y) (`KismetMathLibrary.BreakVector` (`self.K2_GetActorLocation`)))
  (bind _returnvalue (`NiagaraFunctionLibrary.SpawnSystemAtLocation` "/Game/LMH/Effect/smoke_MH.smoke_MH" (`self.K2_GetActorLocation`)))
  (bind (_outhit _returnvalue_2) (`KismetSystemLibrary.LineTraceSingle` (`self.K2_GetActorLocation`) (`KismetMathLibrary.MakeVector` _returnvalue_x _returnvalue_y) "TraceTypeQuery1"))
  (if _returnvalue_2
    (bind (_direction _newtrack_0) (`Timeline|Timeline_0` :!via `PlayFromStart`)
      (:`Update`
        (`self.K2_SetActorLocation` (`KismetMathLibrary.VLerp` (`self.K2_GetActorLocation`) (`.ImpactPoint` (`GameplayStatics.BreakHitResult` _outhit)) _newtrack_0))))
    (else
      (bind (_direction_2 _newtrack_0_2) (`Timeline|Timeline` :!via `PlayFromStart`)
        (:`Update`
          (`self.K2_SetActorLocation` (`KismetMathLibrary.VLerp` (`self.K2_GetActorLocation`) (`.TraceEnd` (`GameplayStatics.BreakHitResult` _outhit)) _newtrack_0_2)))))))

(fn `UserConstructionScript`)