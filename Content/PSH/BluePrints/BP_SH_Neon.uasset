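; BP_SH_Neon is the Neon character Blueprint, managing mesh visibility, death view and animation montages.
; After a short delay on BeginPlay, the local player sees Mesh and others see FpsMesh, which acts as the third-person body despite its name.
; Death montages play on both meshes, while the local view blends to the DeathCamera child actor and reveals FpsMesh.
; Skill and fire events play montages on FpsMesh, and Tick syncs weapon visibility to HasWeapon.
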(event `self.ReceiveBeginPlay`
  (bind _returnvalue (`self.GetController` self))
  (`KismetSystemLibrary.Delay` 0.3)
  (`/Engine/EditorBlueprintResources/StandardMacros.IsValid` _returnvalue
    (:`Is Valid`
      (if (`Controller.IsLocalPlayerController` _returnvalue)
        (`SceneComponent.SetVisibility` (`self.fpsMesh`) false false)
        (`SceneComponent.SetVisibility` (`self.Mesh`) true false)
        (else
          (`SceneComponent.SetVisibility` (`self.fpsMesh`) true false)
          (`SceneComponent.SetVisibility` (`self.Mesh`) false false))))
    (:`Is Not Valid`
      (`SceneComponent.SetVisibility` (`self.fpsMesh`) true false)
      (`SceneComponent.SetVisibility` (`self.Mesh`) false false))))

(event `self.MeshVisible`
  (bind _followcamera (`self.FollowCamera`))
  (bind _deathcamera (`self.DeathCamera`))
  (`/Engine/EditorBlueprintResources/StandardMacros.IsValid` _followcamera
    (:`Is Valid`
      (`ActorComponent.Activate` _followcamera false)
      (`/Engine/EditorBlueprintResources/StandardMacros.IsValid` _deathcamera
        (:`Is Valid`
          (`ActorComponent.Deactivate` _deathcamera)
          (`/Engine/EditorBlueprintResources/StandardMacros.IsValid` (`self.fpsMesh`)
            (:`Is Valid`
              (`SceneComponent.SetVisibility` (`self.Mesh`) false false)
              (`SceneComponent.SetVisibility` (`self.fpsMesh`) false false))))))))

(event `self.PlayDieMontage`
  (if (`self.IsLocallyControlled`)
    (`PlayerController.SetViewTargetWithBlend` (`GameplayStatics.GetPlayerController` 0) (`ChildActorComponent.ChildActor` (`self.DeathCamera`)) 1.0 "VTBlend_EaseInOut" 1.0 false)
    (`SceneComponent.SetVisibility` (`self.fpsMesh`) true false))
  (`|PlayMontage` (`self.fpsMesh`) "/Game/SB/SH_Anim/AM_SH_Die.AM_SH_Die"
    (:`then`
      (`|PlayMontage` (`self.Mesh`) "/Game/SB/SH_Anim/AM_SH_Die.AM_SH_Die"))))

(event `self.ReceiveTick`
  (params (DeltaSeconds :type "Float (single-precision)"))
  (if (`self.HasWeapon`)
    (`SceneComponent.SetVisibility` (`self.BaseWeapon`) true false)
    (else
      (`SceneComponent.SetVisibility` (`self.BaseWeapon`) false false))))

(event `self.BP_Play_1P_Skill_Q_Animation`
  (`|PlayMontage` (`self.fpsMesh`) "/Game/PSH/anim/3P/MT_3P_Skill_Q.MT_3P_Skill_Q"))

(event `self.BP_Play_3P_Skill_C_Animation`
  (`|PlayMontage` (`self.fpsMesh`) "/Game/PSH/anim/3P/MT_3P_skill_C.MT_3P_skill_C"))

(event `self.BP_Play_3p_FireMontage`
  (`|PlayMontage` (`self.fpsMesh`) "/Game/PSH/anim/3P/MT_3P_Fire.MT_3P_Fire"))

(fn `UserConstructionScript`)