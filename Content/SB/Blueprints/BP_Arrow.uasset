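; Sova-style recon arrow projectile that bounces, then releases repeated scan pulses and destroys itself.
; The server aligns the arrow to its velocity and counts time-debounced hits; exceeding the bounce limit disables gravity and physics and multicasts the scan.
; Authority spawns BP_ScanObj, while each machine animates radius timelines into material parameter collections, using separate owner or enemy parameters depending on whether local player 0 owns the arrow.
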(event `self.ReceiveBeginPlay`
  (`MovementComponent.SetUpdatedComponent` (`self.projectileComp`) (`self.Sphere`)))

(event `self.ReceiveTick`
  (params (DeltaSeconds :type "Float (single-precision)"))
  (`|ExecutionSequence`
    (:`then_0`
      (if (`self.HasAuthority`)
        (if (not (> (`self.currBounceCount`) (`self.maxBounceCount`)))
          (`SceneComponent.K2_SetWorldRotation` (`self.ArrowHead`) (`KismetMathLibrary.Conv_VectorToRotator` (`KismetMathLibrary.Normal` (`self.GetVelocity`))) false false)
          (`SceneComponent.K2_SetWorldRotation` (`self.sovaArrow`) (`KismetMathLibrary.Conv_VectorToRotator` (`KismetMathLibrary.Normal` (`self.GetVelocity`))) false false))))
    (:`then_1`
      (if (`self.bHit`)
        (bind _output_get (set `self.currTime` (+ DeltaSeconds (`self.currTime`))))
        (if (> _output_get (`self.DelayTime`))
          (set `self.bHit` false))
        (else
          (set `self.currTime` 0.0))))))

(event `self.Sphere.OnComponentHit`
  (params (HitComponent :type "PrimitiveComponent Object Reference") (OtherActor :type "Actor Object Reference") (OtherComp :type "PrimitiveComponent Object Reference") (NormalImpulse :type "Vector Structure") (Hit :type "HitResult Structure (by ref)"))
  (bind _currbouncecount (`self.currBounceCount`))
  (bind _sphere (`self.Sphere`))
  (`/Engine/EditorBlueprintResources/ActorMacros.Switch Has Authority`
    (:`Authority`
      (if (not (`self.bHit`))
        (set `self.bHit` true)
        (`/Engine/EditorBlueprintResources/StandardMacros.IncrementInt` _currbouncecount
          (:`  `
            (if (> _currbouncecount (`self.maxBounceCount`))
              (set `ProjectileMovementComponent.ProjectileGravityScale` 0.0 (`self.projectileComp`))
              (`PrimitiveComponent.SetEnableGravity` _sphere false)
              (`PrimitiveComponent.SetSimulatePhysics` _sphere false)
              (`self.ServerSpawnScanObj`))))))))

(event `ServerSpawnScanObj`
  (`self.MulticastSpawnScanObj`))

(event `MulticastSpawnScanObj`
  (bind _returnvalue (`self.GetTransform`))
  (`/Engine/EditorBlueprintResources/ActorMacros.Switch Has Authority`
    (:`Authority`
      (`KismetSystemLibrary.PrintString` "arrow" true true (struct :`G` 0.66 :`B` 1.0 :`A` 1.0) 9.0)
      (bind _returnvalue_2 (`|SpawnActorFromClass` "/Game/SB/Blueprints/BP_ScanObj.BP_ScanObj_C" _returnvalue "Undefined" "MultiplyWithRoot" null null))
      (`self.SetOwner` _returnvalue_2 (`self.GetOwner`)))
    (:`Remote`
      _))
  (if (== (`self.GetOwner`) (`GameplayStatics.GetPlayerPawn` 0))
    (`KismetMaterialLibrary.SetVectorParameterValue` "/Game/SB/Materials/PC_ScanPos.PC_ScanPos" "ScanPos" (make `LinearColor` (.x (.location _returnvalue)) (.y (.location _returnvalue)) (.z (.location _returnvalue)) 1.0))
    (bind (_direction _radius) (`Timeline|ScanRadiusEffect` :!via `PlayFromStart` :!label _label)
      (:`Update`
        (`KismetMaterialLibrary.SetScalarParameterValue` "/Game/SB/Materials/PC_Radius.PC_Radius" "Radius" _radius))
      (:`Finished`
        (bind _result (`/Engine/EditorBlueprintResources/StandardMacros.IncrementInt` (`self.waveCount`))
          (:`  `
            (if (< _result 3)
              (goto _label :!via `PlayFromStart`)
              (else
                (`KismetMaterialLibrary.SetScalarParameterValue` "/Game/SB/Materials/PC_Radius.PC_Radius" "Radius")
                (`KismetSystemLibrary.Delay` 0.8)
                (`self.K2_DestroyActor` _returnvalue_2)
                (`self.K2_DestroyActor`)))))))
    (else
      (`KismetMaterialLibrary.SetVectorParameterValue` "/Game/SB/Materials/PC_ScanPos.PC_ScanPos" "EnemyScanPos" (make `LinearColor` (.x (.location _returnvalue)) (.y (.location _returnvalue)) (.z (.location _returnvalue)) 1.0))
      (bind (_direction_2 _radius_2) (`Timeline|Timeline` :!via `PlayFromStart` :!label _label_2)
        (:`Update`
          (`KismetMaterialLibrary.SetScalarParameterValue` "/Game/SB/Materials/PC_Radius.PC_Radius" "EnemyRadius" _radius_2))
        (:`Finished`
          (bind _result_2 (`/Engine/EditorBlueprintResources/StandardMacros.IncrementInt` (`self.waveCount`))
            (:`  `
              (if (< _result_2 3)
                (goto _label_2 :!via `PlayFromStart`)
                (else
                  (`KismetMaterialLibrary.SetScalarParameterValue` "/Game/SB/Materials/PC_Radius.PC_Radius" "EnemyRadius")
                  (`KismetSystemLibrary.Delay` 0.8)
                  (`self.K2_DestroyActor`)
                  (`self.K2_DestroyActor`))))))))))

(fn `UserConstructionScript`)