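; BP_DragonArrow is an actor, apparently a dragon arrow for the Sova character, that hosts a child actor.
; On BeginPlay it passes its own owner to the child actor as that actor's owner.
; An unconnected branch would play a spark sound, in 2D for a locally controlled Sova owner and at the arrow's location otherwise, but it never runs.
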(event `self.ReceiveBeginPlay`
  (`self.SetOwner` (`ChildActorComponent.ChildActor` (`self.ChildActorComp`)) (`self.GetOwner`)))

(fn `UserConstructionScript`)