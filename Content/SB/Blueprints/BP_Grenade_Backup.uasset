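; Backup Blueprint of a throwable grenade that explodes after its first impact.
; Throw runs once, detaching it, launching it via ProjectileMovement and spinning the mesh, then hands velocity to server-simulated physics after a short delay.
; The first authority-side hit fires OnExplosion, routed through server and multicast events to a delayed particle burst, mesh hide and timed cleanup.
; No damage is applied here; debug sphere and prints remain.
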(event `self.ReceiveBeginPlay`
  (add `self.OnExplosion` (delegate `Explosion`)))

(event `Server_Explosion`
  (`self.Multicast_Explosion`))

(event `Explosion`
  (`self.Server_Explosion`))

(event `self.ReceiveTick`
  (params (DeltaSeconds :type "Float (single-precision)"))
  (`KismetSystemLibrary.DrawDebugSphere` (`self.K2_GetActorLocation`) 10.0 12 (struct :`R` 1.0 :`G` 1.0 :`B` 1.0 :`A` 1.0) 0.2 3.0))

(event `Multicast_Explosion`
  (`KismetSystemLibrary.Delay` 0.7)
  (`GameplayStatics.SpawnEmitterAtLocation` "/Game/StarterContent/Particles/P_Explosion.P_Explosion" (`self.K2_GetActorLocation`) (`self.K2_GetActorRotation`) (7.0 7.0 7.0))
  (`KismetSystemLibrary.PrintString` "BOOM!!")
  (`SceneComponent.SetHiddenInGame` (`self.SM_Grenade`) true false)
  (`self.SetLifeSpan` 3.0))

(event `Throw`
  (params (Velocity :type "Vector Structure"))
  (bind _root (`self.Root`))
  (bind _projectilemovement (`self.ProjectileMovement`))
  (`/Engine/EditorBlueprintResources/StandardMacros.DoOnce` false
    (:`Completed`
      (`|ExecutionSequence`
        (:`then_0`
          (`self.K2_DetachFromActor` "KeepWorld" "KeepWorld" "KeepWorld")
          (set `MovementComponent.Velocity` Velocity _projectilemovement)
          (`ActorComponent.Activate` _projectilemovement false)
          (`KismetSystemLibrary.Delay` 0.3)
          (`PrimitiveComponent.SetCollisionEnabled` (`self.Root`) "QueryAndPhysics")
          (bind _output_get (set `self.Velocity` (`self.GetVelocity`)))
          (`/Engine/EditorBlueprintResources/ActorMacros.Switch Has Authority`
            (:`Authority`
              (`PrimitiveComponent.SetSimulatePhysics` _root true)
              (`PrimitiveComponent.SetPhysicsLinearVelocity` _root _output_get false "None"))))
        (:`then_1`
          (`KismetSystemLibrary.MoveComponentTo` (`self.SM_Grenade`) (0.0 0.0 0.0) (`KismetMathLibrary.RandomRotator` false) false false 0.5))))))

(event `self.Root.OnComponentHit`
  (params (HitComponent :type "PrimitiveComponent Object Reference") (OtherActor :type "Actor Object Reference") (OtherComp :type "PrimitiveComponent Object Reference") (NormalImpulse :type "Vector Structure") (Hit :type "HitResult Structure (by ref)"))
  (`/Engine/EditorBlueprintResources/ActorMacros.Switch Has Authority`
    (:`Authority`
      (if (not (`self.HitCheck`))
        (set `self.HitCheck` true)
        (`KismetSystemLibrary.PrintString` "Hit Check Complete")
        (`self.OnExplosion`)))))

(fn `UserConstructionScript`)