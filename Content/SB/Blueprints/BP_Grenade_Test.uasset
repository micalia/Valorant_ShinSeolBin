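; Test grenade actor that can be thrown once and explodes with a particle effect.
; Throw detaches it, launches it with projectile movement plus a random spin, then shortly hands its velocity to physics simulation on the authority.
; OnExplosion routes through server to multicast for a delayed blast, mesh hide and timed destruction.
; The hit check that fires OnExplosion is disconnected, so nothing here triggers it.
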(event `self.ReceiveTick`
  (params (DeltaSeconds :type "Float (single-precision)")))

(event `self.ReceiveBeginPlay`
  (add `self.OnExplosion` (delegate `Explosion`)))

(event `Server_Explosion`
  (`self.Multicast_Explosion`))

(event `Explosion`
  (`self.Server_Explosion`))

(event `Multicast_Explosion`
  (`KismetSystemLibrary.Delay` 0.7)
  (`GameplayStatics.SpawnEmitterAtLocation` "/Game/StarterContent/Particles/P_Explosion.P_Explosion" (`self.K2_GetActorLocation`) (`self.K2_GetActorRotation`) (7.0 7.0 7.0))
  (`KismetSystemLibrary.PrintString` "BOOM!!")
  (`SceneComponent.SetHiddenInGame` (`self.GrenadeMeshComp`) true false)
  (`self.SetLifeSpan` 3.0))

(event `Throw`
  (params (Velocity :type "Vector Structure"))
  (bind _rootcomp (`self.RootComp`))
  (bind _projectilecomp (`self.ProjectileComp`))
  (`/Engine/EditorBlueprintResources/StandardMacros.DoOnce` false
    (:`Completed`
      (`|ExecutionSequence`
        (:`then_0`
          (`self.K2_DetachFromActor` "KeepWorld" "KeepWorld" "KeepWorld")
          (set `MovementComponent.Velocity` Velocity _projectilecomp)
          (`ActorComponent.Activate` _projectilecomp false)
          (`KismetSystemLibrary.Delay` 0.3)
          (`PrimitiveComponent.SetCollisionEnabled` _rootcomp "QueryAndPhysics")
          (bind _output_get (set `self.Velocity` (`self.GetVelocity`)))
          (`/Engine/EditorBlueprintResources/ActorMacros.Switch Has Authority`
            (:`Authority`
              (`PrimitiveComponent.SetSimulatePhysics` _rootcomp true)
              (`PrimitiveComponent.SetPhysicsLinearVelocity` _rootcomp _output_get false "None"))))
        (:`then_1`
          (`KismetSystemLibrary.MoveComponentTo` null (0.0 0.0 0.0) (`KismetMathLibrary.RandomRotator` false) false false 0.5))))))

(fn `UserConstructionScript`)