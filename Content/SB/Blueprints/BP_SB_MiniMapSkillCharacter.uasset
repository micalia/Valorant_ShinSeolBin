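; BP_SB_MiniMapSkillCharacter is a character Blueprint that prototypes a minimap-based smoke skill.
; On BeginPlay it creates the WB_SovaHUD widget, stores it and adds it to the viewport.
; The E-key Enhanced Input action toggles the ActiveSmokeSkill flag and prints a debug message.
; Nodes for image sizing and for showing or hiding a widget with matching cursor and input mode changes are present but unconnected.
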(event `self.ReceiveBeginPlay`
  (bind _returnvalue (`|CreateWidget` "/Game/SB/UMG/WB_SovaHUD.WB_SovaHUD_C"))
  (bind _output_get (set `self.SovaHUD` _returnvalue))
  (`UserWidget.AddToViewport` _output_get 0))

(event `EnhancedInput|/Game/ThirdPerson/Input/Actions/IA_Key_E`
  (params (ActionValue :type Boolean) (ElapsedSeconds :type "Float (double-precision)") (TriggeredSeconds :type "Float (double-precision)") (InputAction :type "InputAction Object Reference" :default "/Game/ThirdPerson/Input/Actions/IA_Key_E.IA_Key_E"))
  (:`Started`
    (`KismetSystemLibrary.PrintString` "E click")
    (if (not (`self.bActiveSmokeSkill`))
      (set `self.bActiveSmokeSkill` true)
      (else
        (set `self.bActiveSmokeSkill` false)))))

(event `EnhancedInput|/Game/ThirdPerson/Input/Actions/IA_MouseLeft`
  (params (ActionValue :type Boolean) (ElapsedSeconds :type "Float (double-precision)") (TriggeredSeconds :type "Float (double-precision)") (InputAction :type "InputAction Object Reference" :default "/Game/ThirdPerson/Input/Actions/IA_MouseLeft.IA_MouseLeft")))

(fn `UserConstructionScript`)