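; Sova character Blueprint with first- and third-person meshes, a death camera, and grenade, air smoke and scouting arrow skill support.
; Grenades spawn on hand sockets by multicast and launch on authority, with the predicted arc drawn as spline meshes.
; Tick hides the weapon during scouting arrow and moves the smoke marker to the cursor; smoke objects spawn server-side.
; Much skill input logic, including arrow firing and smoke targeting, is disconnected.
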(event `self.ReceiveBeginPlay`
  (bind _returnvalue (`self.GetController` self))
  (`KismetSystemLibrary.Delay` 0.3)
  (`/Engine/EditorBlueprintResources/StandardMacros.IsValid` _returnvalue
    (:`Is Valid`
      (if (`Controller.IsLocalPlayerController` _returnvalue)
        (`SceneComponent.SetVisibility` (`self.Mesh`) false false)
        (`SceneComponent.SetVisibility` (`self.fpsMesh`) true false)
        (else
          (`SceneComponent.SetVisibility` (`self.Mesh`) true false)
          (`SceneComponent.SetVisibility` (`self.fpsMesh`) false false))))
    (:`Is Not Valid`
      (`SceneComponent.SetVisibility` (`self.Mesh`) true false)
      (`SceneComponent.SetVisibility` (`self.fpsMesh`) false false))))

(event `self.PlayFpsMontage`
  (`|PlayMontage` (`self.fpsMesh`) "/Game/SB/Animations/Gun/AM_MainFire.AM_MainFire"))

(event `self.ReceiveTick`
  (params (DeltaSeconds :type "Float (single-precision)"))
  (`|ExecutionSequence`
    (:`then_1`
      (if (`self.bScoutingArrow`)
        (`SceneComponent.SetVisibility` (`self. BaseWeapon`) false false)
        (else
          (`SceneComponent.SetVisibility` (`self. BaseWeapon`) true false)))
      (`self.AirSmokeMouseCursor`))))

(event `EnhancedInput|/Game/ThirdPerson/Input/Actions/IA_MouseRight`
  (params (ActionValue :type Boolean) (ElapsedSeconds :type "Float (double-precision)") (TriggeredSeconds :type "Float (double-precision)") (InputAction :type "InputAction Object Reference" :default "/Game/ThirdPerson/Input/Actions/IA_MouseRight.IA_MouseRight"))
  ;[1 1 1] 공중연막 활성화
)

(event `EnhancedInput|/Game/ThirdPerson/Input/Actions/IA_MouseLeft`
  (params (ActionValue :type Boolean) (ElapsedSeconds :type "Float (double-precision)") (TriggeredSeconds :type "Float (double-precision)") (InputAction :type "InputAction Object Reference" :default "/Game/ThirdPerson/Input/Actions/IA_MouseLeft.IA_MouseLeft")))

(event `self.PlaySound`
  (`GameplayStatics.PlaySound2D` "/Game/PSH/SMG/SMG_Cue.SMG_Cue" 1.0 1.0 0.0 null null))

(event `Server_SpawnSmokeObj`
  (params (spawnPos :type "Vector Structure"))
  (`/Engine/EditorBlueprintResources/ActorMacros.Switch Has Authority`
    (:`Authority`
      (bind _returnvalue (`|SpawnActorFromClass` "/Game/SB/Blueprints/BP_SpawnSmokeObj.BP_SpawnSmokeObj_C" (`KismetMathLibrary.MakeTransform` spawnPos) "Undefined" "MultiplyWithRoot" null null))
      (`self.SetOwner` _returnvalue self))))

(event `self.MeshVisible`
  (bind _followcamera (`self.FollowCamera`))
  (bind _deathcamera (`self.DeathCamera`))
  (bind _mesh (`self.Mesh`))
  (`/Engine/EditorBlueprintResources/StandardMacros.IsValid` _followcamera
    (:`Is Valid`
      (`ActorComponent.Activate` _followcamera false)
      (`/Engine/EditorBlueprintResources/StandardMacros.IsValid` _deathcamera
        (:`Is Valid`
          (`ActorComponent.Deactivate` _deathcamera)
          (`/Engine/EditorBlueprintResources/StandardMacros.IsValid` _mesh
            (:`Is Valid`
              (`SceneComponent.SetVisibility` _mesh false false))))))))

(event `self.Fire`
  ;[1 1 1] 정찰용 화살
)

(event `self.PlayDieMontage`
  (if (`self.IsLocallyControlled`)
    (`PlayerController.SetViewTargetWithBlend` (`GameplayStatics.GetPlayerController` 0) (`ChildActorComponent.ChildActor` (`self.DeathCamera`)) 1.0 "VTBlend_EaseInOut" 1.0 false)
    (`SceneComponent.SetVisibility` (`self.Mesh`) true false))
  (`|PlayMontage` (`self.Mesh`) "/Game/LMH/Animation/Standing_React_Death_Backward1_Montage.Standing_React_Death_Backward1_Montage"
    (:`then`
      (`|PlayMontage` (`self.fpsMesh`) "/Game/LMH/Animation/Standing_React_Death_Backward1_Montage.Standing_React_Death_Backward1_Montage"))))

(event `ShowProjectilePath`
  (bind _splinemeshcomponents (`self.SplineMeshComponents`))
  (bind _projectilepath (`self.ProjectilePath`))
  ;[1 1 1] 수류탄
  (`SplineComponent.ClearSplinePoints` (`self.ProjectilePath`) true)
  (for _array_element _splinemeshcomponents
    (`ActorComponent.K2_DestroyComponent` _array_element))
  (`KismetArrayLibrary.Array_Clear` _splinemeshcomponents)
  (if (`self.Throwing`)
    (bind (_outhit _outpathpositions) (`GameplayStatics.Blueprint_PredictProjectilePath_ByTraceChannel` (`SceneComponent.K2_GetComponentLocation` (`self.projectileComp`)) (`self.ThrowVelocity`) true 0.0 "ECC_Camera" false (`|MakeArray` self :!type "Actor Object Reference") "None" 0.0 15.0 3.0))
    (for (_array_element_2 _array_index) _outpathpositions
      (`SplineComponent.AddSplinePointAtIndex` (`self.ProjectilePath`) _array_element_2 _array_index "Local" true))
    (for _index (range (+ (- (`SplineComponent.GetNumberOfSplinePoints` (`self.ProjectilePath`)) 2) 1))
      (bind _returnvalue (`AddComponent|NODE_AddSplineMeshComponent-0` :`bManualAttachment` true))
      (bind _returnvalue_2 (+ _index 1))
      (`SplineMeshComponent.SetStartAndEnd` _returnvalue (`SplineComponent.GetLocationAtSplinePoint` _projectilepath _index "Local") (`SplineComponent.GetTangentAtSplinePoint` _projectilepath _index "Local") (`SplineComponent.GetLocationAtSplinePoint` _projectilepath _returnvalue_2 "Local") (`SplineComponent.GetTangentAtSplinePoint` _projectilepath _returnvalue_2 "Local") true)
      (`KismetArrayLibrary.Array_Add` (`self.SplineMeshComponents`) _returnvalue))
    (`KismetSystemLibrary.Delay` (`GameplayStatics.GetWorldDeltaSeconds`))
    (`self.ShowProjectilePath`)))

(event `self.CancelGrenade`
  ;[1 1 1] 수류탄
  ;;[1 1 1] CancelGrenade
)

(event `Setver_ThrowReady`
  ;[1 1 1] 수류탄
  (`self.Multicast_ThrowReady`))

(event `self.GrenadeThrowReady`
  ;[1 1 1] 수류탄
)

(event `Multicast_ThrowReady`
  ;[1 1 1] 수류탄
)

(event `Server_SpawnGrenade`
  ;[1 1 1] 수류탄
  (`self.Multicast_SpawnGrenade`))

(event `self.DebugSphere`
  ;[1 1 1] 수류탄
)

(event `Multicast_SpawnGrenade`
  ;[1 1 1] 수류탄
  (if (`Controller.IsLocalController` (`GameplayStatics.GetPlayerController` 0))
    (bind _returnvalue (`|SpawnActorFromClass` "/Game/SB/Blueprints/BP_Grenade.BP_Grenade_C" (`KismetMathLibrary.MakeTransform` (`SceneComponent.GetSocketLocation` (`self.fpsMesh`) "Grenade")) "AlwaysSpawn" "MultiplyWithRoot" null null))
    (bind _output_get (set `self.BP_Grenade` _returnvalue))
    (`SceneComponent.K2_AttachToComponent` (`Grenade.RootComp` _output_get) (`self.fpsMesh`) "Grenade" "SnapToTarget" "SnapToTarget" "KeepWorld" true)
    (`self.SetOwner` _returnvalue self)
    (else
      (bind _returnvalue_2 (`|SpawnActorFromClass` "/Game/SB/Blueprints/BP_Grenade.BP_Grenade_C" (`KismetMathLibrary.MakeTransform` (`SceneComponent.GetSocketLocation` (`self.Mesh`) "Grenade")) "AlwaysSpawn" "MultiplyWithRoot" null null))
      (bind _output_get_2 (set `self.BP_Grenade` _returnvalue_2))
      (`SceneComponent.K2_AttachToComponent` (`Grenade.RootComp` _output_get_2) (`self.Mesh`) "Grenade" "SnapToTarget" "SnapToTarget" "KeepWorld" true)
      (`self.SetOwner` _returnvalue_2 self))))

(event `self.GrenadeThrowAction`
  ;[1 1 1] 수류탄
  (`self.Server_GrenadeThrowAction`))

(event `Server_GrenadeThrowAction`
  (bind _bp_grenade (`self.BP_Grenade`))
  (bind _bp_grenade_2 (`self.BP_Grenade`))
  (if (`self.Throwing`)
    (`self.Multicast_GrenadeThrowAction`)
    (set `self.Throwing` false)
    (`KismetSystemLibrary.Delay` 0.1)
    (`/Engine/EditorBlueprintResources/StandardMacros.IsValid` _bp_grenade
      (:`Is Valid`
        (`/Engine/EditorBlueprintResources/ActorMacros.Switch Has Authority`
          (:`Authority`
            (`/Game/SB/Blueprints/BP_Grenade.Throw` _bp_grenade (`self.ThrowVelocity`)))
          (:`Remote`
            _))
        (switch `int` (`KismetMathLibrary.RandomIntegerInRange` 0 1)
          (:`0`
            (`GameplayStatics.PlaySound2D` "/Game/SB/Sounds/Grenade/sova_Grenade0.sova_Grenade0" 1.0 1.0 0.0 null null))
          (:`1`
            (`GameplayStatics.PlaySound2D` "/Game/SB/Sounds/Grenade/sova_Grenade1.sova_Grenade1" 1.0 1.0 0.0 null null)))))
    (else
      (`AnimInstance.Montage_Stop` (`SkeletalMeshComponent.GetAnimInstance` (`self.fpsMesh`)) 0.0 "/Game/SB/Animations/Grenade/AN_SovaGrenade.AN_SovaGrenade")
      (`self.StopAnimMontage` "/Game/SB/Animations/Grenade/AN_SovaGrenade.AN_SovaGrenade")
      (`/Engine/EditorBlueprintResources/StandardMacros.IsValid` _bp_grenade_2
        (:`Is Valid`
          (`self.K2_DestroyActor` _bp_grenade_2))))))

(event `Multicast_GrenadeThrowAction`
  (`KismetSystemLibrary.PrintString` "MultiCast!!")
  (`|PlayMontage` (`self.fpsMesh`) "/Game/SB/Animations/Grenade/AN_SovaGrenade.AN_SovaGrenade" 1.0 0.0 "End"
    (:`then`
      (`|PlayMontage` (`self.Mesh`) "/Game/SB/Animations/Grenade/AN_SovaGrenade.AN_SovaGrenade" 1.0 0.0 "End"))))

(fn `AirSmokeMouseCursor`
  (bind (_locationx _locationy) (`PlayerController.GetMousePosition` (`self.PlayerRef`)))
  (bind (_returnvalue_x _returnvalue_y) (`KismetMathLibrary.BreakVector2D` (* (`Widget.GetDesiredSize` (`self.AirSmokeMarkerRef`)) (/ (`WidgetLayoutLibrary.GetViewportSize`) (1920.0 1080.0)))))
  (bind (_x _y) (`KismetMathLibrary.BreakVector2D` (- (`KismetMathLibrary.MakeVector2D` _locationx _locationy) (/ (`KismetMathLibrary.MakeVector2D` _returnvalue_y _returnvalue_y) (2.0 2.0)))))
  (`/Engine/EditorBlueprintResources/StandardMacros.IsValid` (`self.AirSmokeMarkerRef`)
    (:`Is Valid`
      (`UserWidget.SetPositionInViewport` (`self.AirSmokeMarkerRef`) (`KismetMathLibrary.MakeVector2D` _x _y) true))))

(fn `ClearPathFunc`
  (bind _splinemeshcomponents (`self.SplineMeshComponents`))
  (`SplineComponent.ClearSplinePoints` (`self.ProjectilePath`) true)
  (for _array_element _splinemeshcomponents
    (`ActorComponent.K2_DestroyComponent` _array_element))
  (`KismetArrayLibrary.Array_Clear` _splinemeshcomponents))

(fn `UserConstructionScript`)