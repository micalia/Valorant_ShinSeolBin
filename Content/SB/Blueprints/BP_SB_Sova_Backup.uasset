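; Backup Blueprint of a Sova character prototyping three skills: air smoke, scouting arrow and grenade.
; Air smoke uses a toggled minimap and cursor-following markers, spawning objects at stored locations on right click.
; Grenade montages drive a socket-attached grenade, a predicted spline-mesh path and the throw.
; Much is disconnected: smoke activation and deactivation are empty, and Fire only traces arrow aim, with spawning left unwired.
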(event `self.ReceiveBeginPlay`
  (bind _returnvalue (`|CreateWidget` "/Game/SB/UMG/WB_Proto_SmokeSkillUI.WB_Proto_SmokeSkillUI_C"))
  (bind _output_get (set `self.protoMiniMap` _returnvalue))
  (`UserWidget.AddToViewport` _output_get 0))

(event `Key|Three`
  (params (Key :type "Key Structure"))
  (bind _returnvalue (`GameplayStatics.GetPlayerController` 0))
  (bind _protominimap (`self.protoMiniMap`))
  (:`Pressed`
    (if (`self.On`)
      (set `self.On` false)
      (`Widget.SetVisibility` _protominimap "HitTestInvisible")
      (set `PlayerController.bShowMouseCursor` true _returnvalue)
      (else
        (set `self.On` true)
        (`Widget.SetVisibility` _protominimap "Hidden")
        (set `PlayerController.bShowMouseCursor` false _returnvalue)))))

(event `self.ReceiveTick`
  (params (DeltaSeconds :type "Float (single-precision)"))
  (`self.AirSmokeMouseCursor`))

(event `EnhancedInput|/Game/ThirdPerson/Input/Actions/IA_MouseLeft`
  (params (ActionValue :type Boolean) (ElapsedSeconds :type "Float (double-precision)") (TriggeredSeconds :type "Float (double-precision)") (InputAction :type "InputAction Object Reference" :default "/Game/ThirdPerson/Input/Actions/IA_MouseLeft.IA_MouseLeft"))
  (:`Started`
    (switch `ESovaState` (`self.currState`)
      (:`AirSmoke`
        (if (not (>= (`self.airSmokeCurrCount`) (`self.airSmokeMaxCount`)))
          (bind _returnvalue (`|CreateWidget` "/Game/SB/UMG/WB_AirSmokeMarker.WB_AirSmokeMarker_C"))
          (bind _output_get (set `self.AirSmokeMarkerRef` _returnvalue))
          (`UserWidget.AddToViewport` _output_get 1))))))

(event `EnhancedInput|/Game/ThirdPerson/Input/Actions/IA_MouseRight`
  (params (ActionValue :type Boolean) (ElapsedSeconds :type "Float (double-precision)") (TriggeredSeconds :type "Float (double-precision)") (InputAction :type "InputAction Object Reference" :default "/Game/ThirdPerson/Input/Actions/IA_MouseRight.IA_MouseRight"))
  (:`Started`
    (switch `ESovaState` (`self.currState`)
      (:`AirSmoke`
        (if (> (`self.airSmokeCurrCount`) 0)
          (`|ExecutionSequence`
            (:`then_0`
              (switch `int` (`KismetMathLibrary.RandomIntegerInRange` 0 1)
                (:`0`
                  (`GameplayStatics.PlaySound2D` "/Game/SB/Sounds/AirSmoke/sova_AirSmoke0.sova_AirSmoke0" 1.0 1.0 0.0 null null))
                (:`1`
                  (`GameplayStatics.PlaySound2D` "/Game/SB/Sounds/AirSmoke/sova_AirSmoke1.sova_AirSmoke1" 1.0 1.0 0.0 null null))))
            (:`then_1`
              (for _array_element _
                (`|SpawnActorFromClass` "/Game/SB/Blueprints/BP_ProtoSpawnObj.BP_ProtoSpawnObj_C" (`KismetMathLibrary.MakeTransform` _array_element) "Undefined" "MultiplyWithRoot" null null)))
            (:`then_2`
              (`self.DeactiveAirSmoke`))))))))

(event `self.ActiveAirSmoke`
  ;[1 1 1] 공중 연막
)

(event `self.DeactiveAirSmoke`
  ;[1 1 1] 공중 연막
)

(event `self.Fire`
  (bind _returnvalue (`GameplayStatics.GetPlayerCameraManager` 0))
  (bind _returnvalue_2 (`self.K2_GetActorLocation` _returnvalue))
  ;[1 1 1] 정찰용 화살
  (`|ExecutionSequence`
    (:`then_0`
      ;;[1 1 1] Trace Start Location
      (set `self.CrosshairWorldLocation` _returnvalue_2)
      ;;[1 1 1] Trace End Location
      (set `self.ImpactPoint` (+ _returnvalue_2 (* (`self.GetActorForwardVector` _returnvalue) (15000.0 15000.0 15000.0)))))
    (:`then_1`
      (bind _outhit (`KismetSystemLibrary.LineTraceSingle` (`self.CrosshairWorldLocation`) (`self.ImpactPoint`) "TraceTypeQuery1" false (`|MakeArray` self :!type "Actor Object Reference") "ForDuration"))
      (bind (_bblockinghit _binitialoverlap _time _distance _location _impactpoint) (`GameplayStatics.BreakHitResult` _outhit))
      (if _bblockinghit
        (set `self.ImpactPoint` _impactpoint))
      (set `self.ArrowSpawnLocation` (`SceneComponent.K2_GetComponentLocation` (`self.FirePosMesh`)))
      (set `self.ArrowSpawnRotation` (`KismetMathLibrary.MakeRotFromX` (- (`self.ImpactPoint`) (`self.ArrowSpawnLocation`)))))))

(event `ShowProjectilePath`
  (bind _splinemeshcomponents (`self.SplineMeshComponents`))
  (bind _projectilepath (`self.ProjectilePath`))
  ;[1 1 1] 수류탄
  (`SplineComponent.ClearSplinePoints` (`self.ProjectilePath`) true)
  (for _array_element _splinemeshcomponents
    (`ActorComponent.K2_DestroyComponent` _array_element))
  (`KismetArrayLibrary.Array_Clear` _splinemeshcomponents)
  (if (`self.Throwing`)
    (bind (_outhit _outpathpositions) (`GameplayStatics.Blueprint_PredictProjectilePath_ByTraceChannel` (`SceneComponent.K2_GetComponentLocation` (`self.projectileComp`)) (`self.ThrowVelocity`) true 0.0 "ECC_Camera" false (`|MakeArray` self :!type "Actor Object Reference") "None" 0.0 15.0 3.0))
    (for (_array_element_2 _array_index) _outpathpositions
      (`SplineComponent.AddSplinePointAtIndex` (`self.ProjectilePath`) _array_element_2 _array_index "Local" true))
    (for _index (range (+ (- (`SplineComponent.GetNumberOfSplinePoints` (`self.ProjectilePath`)) 2) 1))
      (bind _returnvalue (`AddComponent|NODE_AddSplineMeshComponent-0` :`bManualAttachment` true))
      (bind _returnvalue_2 (+ _index 1))
      (`SplineMeshComponent.SetStartAndEnd` _returnvalue (`SplineComponent.GetLocationAtSplinePoint` _projectilepath _index "Local") (`SplineComponent.GetTangentAtSplinePoint` _projectilepath _index "Local") (`SplineComponent.GetLocationAtSplinePoint` _projectilepath _returnvalue_2 "Local") (`SplineComponent.GetTangentAtSplinePoint` _projectilepath _returnvalue_2 "Local") true)
      (`KismetArrayLibrary.Array_Add` (`self.SplineMeshComponents`) _returnvalue))
    (`KismetSystemLibrary.Delay` (`GameplayStatics.GetWorldDeltaSeconds`))
    (`self.ShowProjectilePath`)))

(event `self.CancelGrenade`
  (bind _bp_grenade (`self.BP_Grenade`))
  ;[1 1 1] 수류탄
  (`/Engine/EditorBlueprintResources/StandardMacros.IsValid` _bp_grenade
    (:`Is Valid`
      (`self.K2_DestroyActor` _bp_grenade))))

(event `self.GrenadeThrowReady`
  ;[1 1 1] 수류탄
  (`|PlayMontage` (`self.Mesh`) "/Game/SB/Animations/Grenade/AM_Grenade.AM_Grenade"
    (:`then`
      (`|ExecutionSequence`
        (:`then_0`
          (goto _label :!via `Open`))
        (:`then_1`
          (`KismetSystemLibrary.Delay` 0.5)
          (`/Engine/EditorBlueprintResources/StandardMacros.Gate` false :!label _label
            (:`Exit`
              (bind _returnvalue (`|SpawnActorFromClass` "/Game/SB/Blueprints/BP_Grenade.BP_Grenade_C" (`KismetMathLibrary.MakeTransform` (`SceneComponent.GetSocketLocation` (`self.Mesh`) "Grenade")) "AlwaysSpawn" "MultiplyWithRoot" null null))
              (bind _output_get (set `self.BP_Grenade` _returnvalue))
              (`SceneComponent.K2_AttachToComponent` (`/Game/SB/Blueprints/BP_Grenade.Root` _output_get) (`self.Mesh`) "Grenade" "SnapToTarget" "SnapToTarget" "KeepWorld" true))))))
    (:`OnInterrupted`
      (goto _label :!via `Close`))
    (:`OnNotifyBegin`
      (set `self.Throwing` true)
      (`self.ShowProjectilePath`))))

(event `self.ClearPath`
  ;[1 1 1] 수류탄
  (set `self.Throwing` false)
  (`self.StopAnimMontage` "/Game/SB/Animations/Grenade/AM_Grenade.AM_Grenade"))

(event `self.GrenadeThrowAction`
  (bind _bp_grenade (`self.BP_Grenade`))
  (bind _bp_grenade_2 (`self.BP_Grenade`))
  ;[1 1 1] 수류탄
  (if (`self.Throwing`)
    (`|PlayMontage` (`self.Mesh`) "/Game/SB/Animations/Grenade/AM_Grenade.AM_Grenade" 1.0 0.0 "End"
      (:`then`
        (`KismetSystemLibrary.PrintString` "grenade")
        (set `self.Throwing` false)
        (`KismetSystemLibrary.Delay` 0.1)
        (`/Engine/EditorBlueprintResources/StandardMacros.IsValid` _bp_grenade
          (:`Is Valid`
            (`/Game/SB/Blueprints/BP_Grenade.Throw` _bp_grenade (`self.ThrowVelocity`))
            (switch `int` (`KismetMathLibrary.RandomIntegerInRange` 0 1)
              (:`0`
                (`GameplayStatics.PlaySound2D` "/Game/SB/Sounds/Grenade/sova_Grenade0.sova_Grenade0" 1.0 1.0 0.0 null null))
              (:`1`
                (`GameplayStatics.PlaySound2D` "/Game/SB/Sounds/Grenade/sova_Grenade1.sova_Grenade1" 1.0 1.0 0.0 null null)))))))
    (else
      (`self.StopAnimMontage` "/Game/SB/Animations/Grenade/AM_Grenade.AM_Grenade")
      (`/Engine/EditorBlueprintResources/StandardMacros.IsValid` _bp_grenade_2
        (:`Is Valid`
          (`self.K2_DestroyActor` _bp_grenade_2))))))

(fn `AirSmokeMouseCursor`
  (bind (_locationx _locationy) (`PlayerController.GetMousePosition` (`self.PlayerRef`)))
  (bind (_returnvalue_x _returnvalue_y) (`KismetMathLibrary.BreakVector2D` (* (`Widget.GetDesiredSize` (`self.AirSmokeMarkerRef`)) (/ (`WidgetLayoutLibrary.GetViewportSize`) (1920.0 1080.0)))))
  (bind (_x _y) (`KismetMathLibrary.BreakVector2D` (- (`KismetMathLibrary.MakeVector2D` _locationx _locationy) (/ (`KismetMathLibrary.MakeVector2D` _returnvalue_y _returnvalue_y) (2.0 2.0)))))
  (`/Engine/EditorBlueprintResources/StandardMacros.IsValid` (`self.AirSmokeMarkerRef`)
    (:`Is Valid`
      (if (not (>= (`self.airSmokeCurrCount`) (`self.airSmokeMaxCount`)))
        (`UserWidget.SetPositionInViewport` (`self.AirSmokeMarkerRef`) (`KismetMathLibrary.MakeVector2D` _x _y) true)))))

(fn `ClearPathFunc`
  (bind _splinemeshcomponents (`self.SplineMeshComponents`))
  (`SplineComponent.ClearSplinePoints` (`self.ProjectilePath`) true)
  (for _array_element _splinemeshcomponents
    (`ActorComponent.K2_DestroyComponent` _array_element))
  (`KismetArrayLibrary.Array_Clear` _splinemeshcomponents))

(fn `UserConstructionScript`)