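; BP_2DragonArrowSpawn is a short-lived spawner actor that launches a pair of dragon arrows together with a spawn effect.
; On BeginPlay it spawns an enlarged BP_SpawnDragonArrowEffect a fixed distance ahead along its forward vector.
; It then spawns BP_DragonArrow and BP_DragonArrow2 at the transforms of two box components, scaled by EffectScale.
; After a delay the spawner destroys itself.
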(event `self.ReceiveBeginPlay`
  (bind _effectscale (`self.EffectScale`))
  (bind (_returnvalue_location _returnvalue_rotation) (`KismetMathLibrary.BreakTransform` (`SceneComponent.K2_GetComponentToWorld` (`self.Box1`))))
  (bind (_returnvalue_location_2 _returnvalue_rotation_2) (`KismetMathLibrary.BreakTransform` (`SceneComponent.K2_GetComponentToWorld` (`self.Box`))))
  (`|ExecutionSequence`
    (:`then_0`
      (`|SpawnActorFromClass` "/Game/SB/Blueprints/DragonArrow/BP_SpawnDragonArrowEffect.BP_SpawnDragonArrowEffect_C" (`KismetMathLibrary.MakeTransform` (+ (* (`self.GetActorForwardVector`) 1000.0) (`self.K2_GetActorLocation`)) (struct) (4.0 4.0 4.0)) "Undefined" "MultiplyWithRoot" null null))
    (:`then_1`
      (`|SpawnActorFromClass` "/Game/SB/Blueprints/DragonArrow/BP_DragonArrow.BP_DragonArrow_C" (`KismetMathLibrary.MakeTransform` _returnvalue_location_2 _returnvalue_rotation_2 (`KismetMathLibrary.MakeVector` _effectscale _effectscale _effectscale)) "Undefined" "OverrideRootScale" null null)
      (`KismetSystemLibrary.Delay` 16.0 :!label _label)
      (`self.K2_DestroyActor`))
    (:`then_2`
      (`|SpawnActorFromClass` "/Game/SB/Blueprints/DragonArrow/BP_DragonArrow2.BP_DragonArrow2_C" (`KismetMathLibrary.MakeTransform` _returnvalue_location _returnvalue_rotation (`KismetMathLibrary.MakeVector` _effectscale _effectscale _effectscale)) "Undefined" "OverrideRootScale" null null)
      (goto _label))))

(fn `UserConstructionScript`)