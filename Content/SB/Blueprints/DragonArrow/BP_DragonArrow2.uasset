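; Dragon arrow effect actor that plays a one-shot skeletal animation with a water trail, then dissolves and destroys itself.
; BeginPlay sets an initial Dissolve parameter and starts Trail, which attaches a particle emitter using the actor as vertex-surface source.
; After a shared delay, mesh and tail switch to a blue dissolve material animated by a timeline, while the trail stops, eye/Niagara effects hide and destruction follows.
; The portal effect and start-visibility fade are unwired.
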(event `WorlDiss`
  (`MeshComponent.SetScalarParameterValueOnMaterials` (`self.SkeletalMesh`) "Dissolve" 0.8)
  (`MeshComponent.SetScalarParameterValueOnMaterials` (`self.Tail`) "Dissolve" 0.8))

(event `self.ReceiveBeginPlay`
  (bind _skeletalmesh (`self.SkeletalMesh`))
  (`SkeletalMeshComponent.PlayAnimation` (`self.SkeletalMesh`) "/Game/SB/Effect/DragonAbility/Anim/CustomAnim.CustomAnim" false)
  (`|ExecutionSequence`
    (:`then_0`
      (`KismetSystemLibrary.Delay` 10.0)
      (`|ExecutionSequence`
        (:`then_0`
          (`PrimitiveComponent.SetMaterial` _skeletalmesh 0 "/Game/SB/Effect/DragonAbility/Mat_IN/M_BlueDiss_IN.M_BlueDiss_IN")
          (bind (_direction _dis) (`Timeline|Dissolve` :!via `PlayFromStart` :!label _label)
            (:`Update`
              (`MeshComponent.SetScalarParameterValueOnMaterials` (`self.SkeletalMesh`) "amount" _dis)
              (`MeshComponent.SetScalarParameterValueOnMaterials` (`self.Tail`) "amount" _dis))))
        (:`then_1`
          (`PrimitiveComponent.SetMaterial` _skeletalmesh 1 "/Game/SB/Effect/DragonAbility/Mat_IN/M_BlueDiss_IN.M_BlueDiss_IN")
          (goto _label :!via `PlayFromStart`))
        (:`then_2`
          (`PrimitiveComponent.SetMaterial` _skeletalmesh 2 "/Game/SB/Effect/DragonAbility/Mat_IN/M_BlueDiss_IN.M_BlueDiss_IN")
          (goto _label :!via `PlayFromStart`))
        (:`then_3`
          (`PrimitiveComponent.SetMaterial` (`self.Tail`) 0 "/Game/SB/Effect/DragonAbility/Mat_IN/M_BlueDiss_IN.M_BlueDiss_IN")
          (goto _label :!via `PlayFromStart`))))
    (:`then_1`
      (bind _returnvalue (`GameplayStatics.SpawnEmitterAttached` "/Game/SB/Effect/DragonAbility/FX/PS/Water/P_WaterTrail.P_WaterTrail" (`self.SkeletalMesh`) "0" (0.0 0.0 0.0) (struct) (1.0 1.0 1.0) "SnapToTargetIncludingScale"))
      (set `ParticleSystemComponent.InstanceParameters` (`|MakeArray` (make `ParticleSysParam` "VertSurfaceActor" "PSPT_Actor" 0.0 0.0 (0.0 0.0 0.0) (0.0 0.0 0.0) (struct) self)) _returnvalue)
      (`KismetSystemLibrary.Delay` 10.0)
      (`ActorComponent.Deactivate` _returnvalue)
      (`|ExecutionSequence`
        (:`then_0`
          (`KismetSystemLibrary.Delay` 1.0)
          (`self.K2_DestroyActor`))
        (:`then_1`
          (`SceneComponent.SetVisibility` (`self.SM_EyeFX`) false false)
          (`SceneComponent.SetVisibility` (`self.Niagara1`) false false)
          (`SceneComponent.SetVisibility` (`self.Niagara`) false false))))
    (:`then_4`
      (`self.WorlDiss`))))

(fn `UserConstructionScript`)