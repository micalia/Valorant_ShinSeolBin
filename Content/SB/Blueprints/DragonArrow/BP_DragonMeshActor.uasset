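; Visual dragon actor owned by SB_Sova, under DragonArrow, that plays a one-shot animation with an attached water-trail emitter.
; On BeginPlay it creates dynamic materials, keeping the default look for the locally controlled owner and tinting red for others.
; After ten seconds it swaps to blue or red dissolve materials driven by a timeline, deactivates the trail, hides effects and destroys itself.
; The portal effect is never called.
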(event `WorlDiss`
  (`MeshComponent.SetScalarParameterValueOnMaterials` (`self.SkeletalMesh`) "Dissolve" 0.8)
  (`MeshComponent.SetScalarParameterValueOnMaterials` (`self.Tail`) "Dissolve" 0.8))

(event `self.ReceiveBeginPlay`
  (bind _matinst2 (`self.MatInst2`))
  (bind _tailmat (`self.TailMat`))
  (bind _skeletalmesh (`self.SkeletalMesh`))
  (bind _skeletalmesh_2 (`self.SkeletalMesh`))
  (bind _tail (`self.Tail`))
  (bind _matinst (`self.MatInst`))
  (bind _skeletalmesh_3 (`self.SkeletalMesh`))
  (bind _returnvalue (`PrimitiveComponent.CreateDynamicMaterialInstance` _skeletalmesh_3 0 (`PrimitiveComponent.GetMaterial` _skeletalmesh_3 0) "None"))
  (set `self.MatInst` _returnvalue)
  (bind _returnvalue_2 (`PrimitiveComponent.CreateDynamicMaterialInstance` _skeletalmesh_3 1 (`PrimitiveComponent.GetMaterial` _skeletalmesh_3 1) "None"))
  (set `self.MatInst2` _returnvalue_2)
  (bind _returnvalue_3 (`PrimitiveComponent.CreateDynamicMaterialInstance` _tail 0 (`PrimitiveComponent.GetMaterial` _tail 0) "None"))
  (set `self.TailMat` _returnvalue_3)
  (bind _assb_sova (cast `SB_Sova` (`self.GetOwner`)))
  (if (`Pawn.IsLocallyControlled` _assb_sova)
    (`SkeletalMeshComponent.PlayAnimation` (`self.SkeletalMesh`) "/Game/SB/Effect/DragonAbility/Anim/CustomAnim.CustomAnim" false :!label _label)
    (`|ExecutionSequence`
      (:`then_0`
        (`KismetSystemLibrary.Delay` 10.0)
        (bind _assb_sova_2 (cast `SB_Sova` (`self.GetOwner`)))
        (if (`Pawn.IsLocallyControlled` _assb_sova_2)
          (`|ExecutionSequence`
            (:`then_0`
              (`PrimitiveComponent.SetMaterial` _skeletalmesh 0 "/Game/SB/Effect/DragonAbility/Mat_IN/M_BlueDiss_IN.M_BlueDiss_IN")
              (bind (_direction _dis) (`Timeline|Dissolve` :!via `PlayFromStart` :!label _label_2)
                (:`Update`
                  (`MeshComponent.SetScalarParameterValueOnMaterials` (`self.SkeletalMesh`) "amount" _dis)
                  (`MeshComponent.SetScalarParameterValueOnMaterials` (`self.Tail`) "amount" _dis))))
            (:`then_1`
              (`PrimitiveComponent.SetMaterial` _skeletalmesh 1 "/Game/SB/Effect/DragonAbility/Mat_IN/M_BlueDiss_IN.M_BlueDiss_IN")
              (goto _label_2 :!via `PlayFromStart`))
            (:`then_2`
              (`PrimitiveComponent.SetMaterial` _skeletalmesh 2 "/Game/SB/Effect/DragonAbility/Mat_IN/M_BlueDiss_IN.M_BlueDiss_IN")
              (goto _label_2 :!via `PlayFromStart`))
            (:`then_3`
              (`PrimitiveComponent.SetMaterial` (`self.Tail`) 0 "/Game/SB/Effect/DragonAbility/Mat_IN/M_BlueDiss_IN.M_BlueDiss_IN")
              (goto _label_2 :!via `PlayFromStart`)))
          (else
            (`|ExecutionSequence`
              (:`then_0`
                (`PrimitiveComponent.SetMaterial` _skeletalmesh_2 0 "/Game/SB/Effect/DragonAbility/Mat_IN/M_RedDiss_IN1.M_RedDiss_IN1"))
              (:`then_1`
                (`PrimitiveComponent.SetMaterial` _skeletalmesh_2 1 "/Game/SB/Effect/DragonAbility/Mat_IN/M_RedDiss_IN1.M_RedDiss_IN1"))
              (:`then_2`
                (`PrimitiveComponent.SetMaterial` _skeletalmesh_2 2 "/Game/SB/Effect/DragonAbility/Mat_IN/M_RedDiss_IN1.M_RedDiss_IN1"))
              (:`then_3`
                (`PrimitiveComponent.SetMaterial` (`self.Tail`) 0 "/Game/SB/Effect/DragonAbility/Mat_IN/M_RedDiss_IN1.M_RedDiss_IN1")
                (goto _label_2 :!via `PlayFromStart`))))))
      (:`then_1`
        (bind _returnvalue_4 (`GameplayStatics.SpawnEmitterAttached` "/Game/SB/Effect/DragonAbility/FX/PS/Water/P_WaterTrail.P_WaterTrail" (`self.SkeletalMesh`) "0" (0.0 0.0 0.0) (struct) (1.0 1.0 1.0) "SnapToTargetIncludingScale"))
        (set `ParticleSystemComponent.InstanceParameters` (`|MakeArray` (make `ParticleSysParam` "VertSurfaceActor" "PSPT_Actor" 0.0 0.0 (0.0 0.0 0.0) (0.0 0.0 0.0) (struct) self)) _returnvalue_4)
        (`KismetSystemLibrary.Delay` 10.0)
        (`ActorComponent.Deactivate` _returnvalue_4)
        (`|ExecutionSequence`
          (:`then_0`
            (`KismetSystemLibrary.Delay` 1.0)
            (`self.K2_DestroyActor`))
          (:`then_1`
            (`SceneComponent.SetVisibility` (`self.SM_EyeFX`) false false)
            (`SceneComponent.SetVisibility` (`self.Niagara1`) false false)
            (`SceneComponent.SetVisibility` (`self.Niagara`) false false))))
      (:`then_4`
        (`self.WorlDiss`)))
    (else
      (`|ExecutionSequence`
        (:`then_0`
          (`MaterialInstanceDynamic.SetTextureParameterValue` _matinst "T-Noise" "/Game/SB/Textures/DragonArrow/T_Water3_Red.T_Water3_Red"))
        (:`then_1`
          (`MaterialInstanceDynamic.SetTextureParameterValue` _matinst "T-NoiseR" "/Game/SB/Textures/DragonArrow/T_Water3_Red.T_Water3_Red"))
        (:`then_2`
          (`MaterialInstanceDynamic.SetVectorParameterValue` _matinst "Color" (struct :`R` 60.0 :`G` 0.045186 :`B` 0.017642 :`A` 1.0)))
        (:`then_4`
          (`MaterialInstanceDynamic.SetTextureParameterValue` _matinst2 "T-Noise" "/Game/SB/Textures/DragonArrow/T_Water3_Red.T_Water3_Red")
          (`MaterialInstanceDynamic.SetTextureParameterValue` _matinst2 "T-NoiseR" "/Game/SB/Textures/DragonArrow/T_Water3_Red.T_Water3_Red")
          (`MaterialInstanceDynamic.SetVectorParameterValue` _matinst2 "Color" (struct :`R` 60.0 :`G` 0.045186 :`B` 0.017642 :`A` 1.0))
          (`MaterialInstanceDynamic.SetTextureParameterValue` _tailmat "T-Noise" "/Game/SB/Textures/DragonArrow/T_Water3_Red.T_Water3_Red")
          (`MaterialInstanceDynamic.SetTextureParameterValue` _tailmat "T-NoiseR" "/Game/SB/Textures/DragonArrow/T_Water3_Red.T_Water3_Red")
          (`MaterialInstanceDynamic.SetVectorParameterValue` _tailmat "Color" (struct :`R` 60.0 :`G` 0.045186 :`B` 0.017642 :`A` 1.0))
          (goto _label))))))

(fn `UserConstructionScript`)