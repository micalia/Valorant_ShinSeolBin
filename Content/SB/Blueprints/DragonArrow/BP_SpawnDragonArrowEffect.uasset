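; BP_SpawnDragonArrowEffect is an effect actor for Sova's Dragon Arrow, going by its name and owner class.
; On BeginPlay it casts its owner to SB_Sova and, when that Sova is not locally controlled, swaps the Fx particle template to P_Red_waterBallHit.
; Locally controlled owners keep the default template, and the actor has no other active logic.
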(event `self.ReceiveBeginPlay`
  (bind _assb_sova (cast `SB_Sova` (`self.GetOwner`)))
  (if (not (`Pawn.IsLocallyControlled` _assb_sova))
    (`ParticleSystemComponent.SetTemplate` (`self.fx`) "/Game/FXVarietyPack/Particles/P_Red_waterBallHit.P_Red_waterBallHit")))

(fn `UserConstructionScript`
  (`parent.UserConstructionScript`))