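; Effect actor for the blue dragon ability's first attack, which plays the one-shot Att1 animation on its skeletal mesh at BeginPlay.
; Trail then attaches a water trail emitter to the mesh, passing the actor as the VertSurfaceActor particle parameter.
; The WorlDiss event is empty, and the dissolve, portal, delayed cleanup and self-destroy logic is unwired, so it never runs.
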(event `WorlDiss`)

(event `self.ReceiveBeginPlay`
  (`|ExecutionSequence`
    (:`then_0`
      (`SkeletalMeshComponent.PlayAnimation` (`self.SkeletalMesh`) "/Game/SB/Effect/DragonAbility/Anim/Att1.Att1" false)
      (`|ExecutionSequence`
        (:`then_1`
          (bind _returnvalue (`GameplayStatics.SpawnEmitterAttached` "/Game/SB/Effect/DragonAbility/FX/PS/Water/P_WaterTrail.P_WaterTrail" (`self.SkeletalMesh`) "0" (0.0 0.0 0.0) (struct) (1.0 1.0 1.0) "SnapToTargetIncludingScale"))
          (set `ParticleSystemComponent.InstanceParameters` (`|MakeArray` (make `ParticleSysParam` "VertSurfaceActor" "PSPT_Actor" 0.0 0.0 (0.0 0.0 0.0) (0.0 0.0 0.0) (struct) self)) _returnvalue))))
    (:`then_2`
      (`self.WorlDiss`))))

(fn `UserConstructionScript`)