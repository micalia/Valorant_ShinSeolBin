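; Effect actor for a dark dragon ability (right-side attack 10) that plays a one-shot attack animation on its skeletal mesh, slightly sped up.
; A Niagara dark trail attaches to the mesh and runs alongside the animation.
; After a fixed delay, the body and tail switch to a dissolve material driven by a timeline, while the trail deactivates and eye and Niagara effects hide.
; The actor destroys itself shortly afterwards.
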(event `self.ReceiveBeginPlay`
  (bind _skeletalmesh (`self.SkeletalMesh`))
  (bind _skeletalmesh_2 (`self.SkeletalMesh`))
  (`SkeletalMeshComponent.PlayAnimation` _skeletalmesh "/Game/SB/Effect/DragonAbility/Anim/Att8R.Att8R" false)
  (`SkeletalMeshComponent.SetPlayRate` _skeletalmesh 1.2)
  (`|ExecutionSequence`
    (:`then_0`
      (`KismetSystemLibrary.Delay` 3.8)
      (`|ExecutionSequence`
        (:`then_0`
          (`PrimitiveComponent.SetMaterial` _skeletalmesh_2 0 "/Game/SB/Effect/DragonAbility/Mat_IN/M_DarkDiss_IN.M_DarkDiss_IN")
          (bind (_direction _dis) (`Timeline|Dissolve` :!label _label)
            (:`Update`
              (`MeshComponent.SetScalarParameterValueOnMaterials` (`self.SkeletalMesh`) "amount" _dis)
              (`MeshComponent.SetScalarParameterValueOnMaterials` (`self.Tail`) "amount" _dis))))
        (:`then_1`
          (`PrimitiveComponent.SetMaterial` _skeletalmesh_2 1 "/Game/SB/Effect/DragonAbility/Mat_IN/M_DarkDiss_IN.M_DarkDiss_IN")
          (goto _label))
        (:`then_2`
          (`PrimitiveComponent.SetMaterial` _skeletalmesh_2 2 "/Game/SB/Effect/DragonAbility/Mat_IN/M_DarkDiss_IN.M_DarkDiss_IN")
          (goto _label))
        (:`then_3`
          (`PrimitiveComponent.SetMaterial` (`self.Tail`) 0 "/Game/SB/Effect/DragonAbility/Mat_IN/M_DarkDiss_IN.M_DarkDiss_IN")
          (goto _label))))
    (:`then_1`
      (bind _returnvalue (`NiagaraFunctionLibrary.SpawnSystemAttached` "/Game/SB/Effect/DragonAbility/FX/NS/Dark/NS_DarkTrail.NS_DarkTrail" (`self.SkeletalMesh`) "None" (0.0 0.0 0.0) (struct) "SnapToTargetIncludingScale" true))
      (`KismetSystemLibrary.Delay` 3.8)
      (`ActorComponent.Deactivate` _returnvalue)
      (`|ExecutionSequence`
        (:`then_0`
          (`KismetSystemLibrary.Delay` 1.0)
          (`self.K2_DestroyActor`))
        (:`then_1`
          (`SceneComponent.SetVisibility` (`self.SM_EyeFX`) false false)
          (`SceneComponent.SetVisibility` (`self.Niagara1`) false false)
          (`SceneComponent.SetVisibility` (`self.Niagara`) false false))))))

(fn `UserConstructionScript`)