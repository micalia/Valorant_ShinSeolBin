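; Effect actor for the blue dragon's second attack ability, playing the Att2 animation once on BeginPlay.
; It immediately attaches a water trail emitter to the skeletal mesh, passing itself as the particle's surface actor.
; After a delay, it swaps the body and tail materials to a blue dissolve material.
; The dissolve timelines, portal effect and trail shutdown with self-destruction are present but unconnected.
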(event `WorlDiss`
  (`KismetSystemLibrary.Delay` 0.3)
  (bind (_direction _vis) (`Timeline|StartVisiblity` :!via `PlayFromStart`)
    (:`Update`
      (`MeshComponent.SetScalarParameterValueOnMaterials` (`self.SkeletalMesh`) "Dissolve" _vis)
      (`MeshComponent.SetScalarParameterValueOnMaterials` (`self.Tail`) "Dissolve" _vis))))

(event `self.ReceiveBeginPlay`
  (bind _skeletalmesh (`self.SkeletalMesh`))
  (`SkeletalMeshComponent.PlayAnimation` (`self.SkeletalMesh`) "/Game/SB/Effect/DragonAbility/Anim/Att2.Att2" false)
  (`|ExecutionSequence`
    (:`then_0`
      (`KismetSystemLibrary.Delay` 3.2)
      (`|ExecutionSequence`
        (:`then_0`
          (`PrimitiveComponent.SetMaterial` _skeletalmesh 0 "/Game/SB/Effect/DragonAbility/Mat_IN/M_BlueDiss_IN.M_BlueDiss_IN"))
        (:`then_1`
          (`PrimitiveComponent.SetMaterial` _skeletalmesh 1 "/Game/SB/Effect/DragonAbility/Mat_IN/M_BlueDiss_IN.M_BlueDiss_IN"))
        (:`then_2`
          (`PrimitiveComponent.SetMaterial` _skeletalmesh 2 "/Game/SB/Effect/DragonAbility/Mat_IN/M_BlueDiss_IN.M_BlueDiss_IN"))
        (:`then_3`
          (`PrimitiveComponent.SetMaterial` (`self.Tail`) 0 "/Game/SB/Effect/DragonAbility/Mat_IN/M_BlueDiss_IN.M_BlueDiss_IN"))))
    (:`then_1`
      (bind _returnvalue (`GameplayStatics.SpawnEmitterAttached` "/Game/SB/Effect/DragonAbility/FX/PS/Water/P_WaterTrail.P_WaterTrail" (`self.SkeletalMesh`) "0" (0.0 0.0 0.0) (struct) (1.0 1.0 1.0) "SnapToTargetIncludingScale"))
      (set `ParticleSystemComponent.InstanceParameters` (`|MakeArray` (make `ParticleSysParam` "VertSurfaceActor" "PSPT_Actor" 0.0 0.0 (0.0 0.0 0.0) (0.0 0.0 0.0) (struct) self)) _returnvalue))))

(fn `UserConstructionScript`)