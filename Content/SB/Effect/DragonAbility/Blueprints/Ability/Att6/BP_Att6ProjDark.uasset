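; Dark projectile actor for the dragon's Att6 ability, built on a looping animated skeletal mesh that explodes on contact.
; On BeginPlay it spawns a portal effect, attaches a Niagara dark trail and runs a timeline driving the Dissolve parameter on the mesh and tail, with a limited lifespan.
; Each tick it sphere-traces at listed mesh sockets; a hit spawns a dark explosion and destroys the actor, with no damage applied here.
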(fn `UserConstructionScript`)