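; BP_Fx is a placeable effect actor that spawns a Cascade emitter and a Niagara system in the world, either once or on a repeating interval.
; On BeginPlay a named timer calls Fx, which waits for a delay, then spawns both effects at the Location component's world position.
; Templates, rotations, scales, timing and looping are all driven by variables, so one Blueprint can serve different effects.
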(event `self.ReceiveBeginPlay`
  (`KismetSystemLibrary.K2_SetTimer` null "Fx" (`self.TimeLoop`) (`self.Looping`)))

(event `Fx`
  (bind _returnvalue (`SceneComponent.K2_GetComponentLocation` (`self.Location`)))
  (`KismetSystemLibrary.Delay` (`self.Delay`))
  (`|ExecutionSequence`
    (:`then_0`
      (`GameplayStatics.SpawnEmitterAtLocation` (`self.Cascade`) _returnvalue (`self.RotationCas`) (`self.ScaleCas`)))
    (:`then_1`
      (`NiagaraFunctionLibrary.SpawnSystemAtLocation` (`self.Niagara`) _returnvalue (`self.RotationNia`) (`self.ScaleNia`)))))

(fn `UserConstructionScript`)