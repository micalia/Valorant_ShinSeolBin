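; BP_RingGrow is an effect Blueprint that endlessly animates two rings, moving and scaling them.
; Each ring slides between its relative origin and a Y offset with chained MoveComponentTo calls, in opposite order to the other.
; In parallel, each ring runs two chained timelines that drive uniform world scale.
; Tick triggers both loops through DoOnce gates, which reset when the movement or scale chain completes.
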(event `self.ReceiveTick`
  (params (DeltaSeconds :type "Float (single-precision)"))
  (`|ExecutionSequence`
    (:`then_0`
      (`self.LoopRing1`))
    (:`then_1`
      (`self.LoopRing2`))))

(event `LoopRing2`
  (bind _ring2 (`self.Ring2`))
  (bind _ring2_2 (`self.Ring2`))
  ;[1 1 1] Ring 2
  (`/Engine/EditorBlueprintResources/StandardMacros.DoOnce` false :!label _label
    (:`Completed`
      (`|ExecutionSequence`
        (:`then_0`
          (`KismetSystemLibrary.MoveComponentTo` _ring2 (0.0 0.0 0.0) (struct) false false 2.0)
          (`KismetSystemLibrary.MoveComponentTo` _ring2 (0.0 -130.0 0.0) (struct) false false 1.0)
          (`self.ResetRing2` :!label _label_2))
        (:`then_1`
          (bind (_direction _scale) (`Timeline|R2Scale1` :!via `PlayFromStart`)
            (:`Update`
              (`SceneComponent.SetWorldScale3D` _ring2_2 (`KismetMathLibrary.MakeVector` _scale _scale _scale)))
            (:`Finished`
              (bind (_direction_2 _scaleb) (`Timeline|R2Scale2` :!via `PlayFromStart`)
                (:`Update`
                  (`SceneComponent.SetWorldScale3D` _ring2_2 (`KismetMathLibrary.MakeVector` _scaleb _scaleb _scaleb)))
                (:`Finished`
                  (goto _label_2))))))))))

(event `ResetRing2`
  ;[1 1 1] Ring 2
  (goto _label :!via `Reset`))

(event `LoopRing1`
  (bind _ring1 (`self.Ring1`))
  (bind _ring1_2 (`self.Ring1`))
  ;[1 1 1] Ring 2
  (`/Engine/EditorBlueprintResources/StandardMacros.DoOnce` false :!label _label_3
    (:`Completed`
      (`|ExecutionSequence`
        (:`then_0`
          (`KismetSystemLibrary.MoveComponentTo` _ring1 (0.0 -130.0 0.0) (struct) false false 2.0)
          (`KismetSystemLibrary.MoveComponentTo` _ring1 (0.0 0.0 0.0) (struct) false false 1.0)
          (`self.ResetRing1` :!label _label_4))
        (:`then_1`
          (bind (_direction _scale) (`Timeline|R1Scale1` :!via `PlayFromStart`)
            (:`Update`
              (`SceneComponent.SetWorldScale3D` _ring1_2 (`KismetMathLibrary.MakeVector` _scale _scale _scale)))
            (:`Finished`
              (bind (_direction_2 _scaleb) (`Timeline|R1Scale2` :!via `PlayFromStart`)
                (:`Update`
                  (`SceneComponent.SetWorldScale3D` _ring1_2 (`KismetMathLibrary.MakeVector` _scaleb _scaleb _scaleb)))
                (:`Finished`
                  (goto _label_4))))))))))

(event `ResetRing1`
  ;[1 1 1] Ring 2
  (goto _label_3 :!via `Reset`))

(fn `UserConstructionScript`)